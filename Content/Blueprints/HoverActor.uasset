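; HoverActor is a chess actor that tracks what is under the mouse cursor, with its hover response still unfinished.
; BeginPlay spawns an actor at the origin for each class in the default ChessPieceArrays data table row, storing them in ChessPieces.
; Tick runs a cursor trace, ignores tiles, and maps a hit piece's board index through ChessBoard to a stored actor.
; It only validates that actor and takes no further action.
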(event EventBeginPlay
  (bind _returnvalue (Utilities|GetDataTableRow "/Game/DataTables/ChessPieceArrays.ChessPieceArrays" "ChessPieceDefaultArray")
    (:then
      (for _array_element (Utilities|Struct|BreakChessPieceArray _returnvalue)
        (bind _returnvalue_2 (Game|SpawnActorfromClass _array_element (Math|Transform|MakeTransform "0, 0, 0") "AlwaysSpawn" "MultiplyWithRoot" 0 0))
        (Rendering|SetActorHiddenInGame _returnvalue_2 false)
        (Utilities|Array|Add (Variables|Default|GetChessPieces) _returnvalue_2)))))

(event EventTick
  (params (DeltaSeconds :type Float%20%28single-precision%29))
  (bind _output_get (Variables|Default|SetCurrHoverActor (.HitActor (Collision|BreakHitResult (.HitResult (Game|Player|GetHitResultUnderCursorbyChannel (Game|GetPlayerController 0) "TraceTypeQuery1" true))))))
  (if (Utilities|IsValid _output_get)
    (Utilities|Casting|CastToChessTile _output_get
      (:CastFailed
        (bind _aschess_piece (Utilities|Casting|CastToChessPiece _output_get))
        (bind _pieceindex (Default|GetPieceIndexatBoardIndex (Variables|Default|GetChessBoard) (Variables|/Game/Blueprints/ChessPiece.ChessPiece_C|GetBoardIndex _aschess_piece)))
        (if (Utilities|IsValid (Utilities|Array|Get(acopy) (Variables|Default|GetChessPieces) _pieceindex))
          _)))))

(fn ConstructionScript)