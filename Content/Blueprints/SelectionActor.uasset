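; Selection actor for a chess game that shows a hover preview of the tile or piece under the cursor.
; On BeginPlay it spawns a hidden, collision-free ghost of each data-table piece class plus a tile, using the SelectionPreview material.
; While the board's game state is not idle, Tick traces under the cursor and moves the matching ghost onto the hit actor.
; Click selection is unfinished, only clearing and printing the selection variables.
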(event EventBeginPlay
  (Utilities|FlowControl|Sequence
    (:then_0
      (bind _returnvalue (Utilities|GetDataTableRow "/Game/DataTables/ChessPieceArrays.ChessPieceArrays" "ChessPieceDefaultArray")
        (:then
          (Utilities|Array|Resize (Variables|Default|GetChessPieces) (Utilities|Array|Length (Utilities|Struct|BreakChessPieceArray _returnvalue)))
          (for (_array_element _array_index) (Utilities|Struct|BreakChessPieceArray _returnvalue)
            (if (Utilities|IsValidClass _array_element)
              (bind _spawnedactor (CallFunction|SpawnHoverSelectionActor _array_element true))
              (bind _aschess_piece (Utilities|Casting|CastToChessPiece _spawnedactor))
              (CallFunction|SetupHoverSelectionStaticMesh (Variables|/Game/Blueprints/ChessPiece.ChessPiece_C|GetStaticMesh _aschess_piece))
              (Utilities|Array|SetArrayElem (Variables|Default|GetChessPieces) _array_index _aschess_piece))))))
    (:then_1
      (bind _spawnedactor_2 (CallFunction|SpawnHoverSelectionActor "/Game/Blueprints/ChessTile.ChessTile_C" true))
      (bind _aschess_tile (Utilities|Casting|CastToChessTile _spawnedactor_2))
      (CallFunction|SetupHoverSelectionStaticMesh (Variables|/Game/Blueprints/ChessTile.ChessTile_C|GetCube _aschess_tile))
      (Variables|Default|SetChessTile _aschess_tile))))

(event EventTick
  (params (DeltaSeconds :type Float%20%28single-precision%29))
  (bind _returnvalue (Game|GetPlayerController 0))
  (bind _hitresult (Game|Player|GetHitResultUnderCursorbyChannel _returnvalue "TraceTypeQuery1" true))
  (bind _hitactor (Collision|BreakHitResult _hitresult))
  (if (|IfGameStateisnotIdle)
    (CallFunction|ResetAllHoverActor)
    (if (Utilities|IsValid _hitactor)
      (bind _aschess_tile (Utilities|Casting|CastToChessTile _hitactor)
        (:then
          (CallFunction|DisplayHoverActor (Variables|Default|GetChessTile) (Transformation|GetActorTransform _aschess_tile)))
        (:CastFailed
          (bind _aschess_piece (Utilities|Casting|CastToChessPiece _hitactor))
          (bind _pieceindex (Default|GetPieceIndexatBoardIndex (Variables|Default|GetChessBoard) (Variables|/Game/Blueprints/ChessPiece.ChessPiece_C|GetBoardIndex _aschess_piece)))
          (if (Utilities|IsValid (Utilities|Array|Get(acopy) (Variables|Default|GetChessPieces) (Math|Integer|Absolute(Integer) _pieceindex)))
            (CallFunction|DisplayHoverActor (Utilities|Array|Get(acopy) (Variables|Default|GetChessPieces) (Math|Integer|Absolute(Integer) _pieceindex)) (Transformation|GetActorTransform _aschess_piece))))))))

(event Input|ActionEvents|InputActionClick
  (params (Key :type Key%20Structure :default "None"))
  ;[1 1 1] Selected (Incomplete)
  (:Pressed
    (bind (_ischesstile _ischesspiece) (CallFunction|ActorType (Variables|Default|GetCurrHoverActor)))
    (if _ischesspiece
      (bind _output_get (Variables|Default|SetSelectedChesPiece 0))
      (Development|PrintString (Utilities|GetDisplayName _output_get))
      (elif _ischesstile
        (bind _output_get_2 (Variables|Default|SetSelectedChessTile 0))
        (Development|PrintString (Utilities|GetDisplayName _output_get_2))))))

(fn ConstructionScript)

(fn SpawnHoverSelectionActor
  (params (ActorClass :type Actor%20Class%20Reference) (Hidden :type Boolean))
  (bind _returnvalue (Game|SpawnActorfromClass ActorClass (Math|Transform|MakeTransform "0, 0, 0") "AlwaysSpawn" "MultiplyWithRoot" 0 0))
  (Rendering|SetActorHiddenInGame _returnvalue Hidden)
  (return _returnvalue))

(fn SetupHoverSelectionStaticMesh
  (params (StaticMeshComp :type Static%20Mesh%20Component%20Object%20Reference))
  (Rendering|Material|SetMaterial StaticMeshComp 0 "/Game/Materials/SelectionPreview.SelectionPreview")
  (Collision|SetCollisionEnabled StaticMeshComp "NoCollision"))

(fn DisplayHoverActor
  (params (HoverActor :type Actor%20Object%20Reference) (TargetTransform :type Transform))
  (Rendering|SetActorHiddenInGame HoverActor false)
  (Transformation|SetActorTransform HoverActor TargetTransform false true)
  (Variables|Default|SetCurrHoverActor HoverActor))

(fn ResetAllHoverActor
  (for _array_element (Variables|Default|GetChessPieces)
    (if (Utilities|IsValid _array_element)
      (Rendering|SetActorHiddenInGame _array_element true)))
  (Rendering|SetActorHiddenInGame (Variables|Default|GetChessTile) true))

(fn ActorType
  (params (ActorToCheck :type Actor%20Object%20Reference))
  (Utilities|Casting|CastToChessPiece ActorToCheck
    (:then
      (return false true))
    (:CastFailed
      (Utilities|Casting|CastToChessTile ActorToCheck
        (:then
          (return true false))
        (:CastFailed
          (return false false))))))