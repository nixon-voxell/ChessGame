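; Chess board Blueprint that handles the presentation side of turn changes and game end.
; Each turn-start event moves the camera transition to the active color's side, then switches the countdown widget to the other player.
; White and Black win events share a helper that stops the music, freezes global time dilation and shows an end menu, which then receives the winner's display name.
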(event EventOnWhiteWin
  (bind _endmenu (Utilities|CreateEndMenu)
    (:executeOut
      (Variables|/Game/HUD/EndMenu.EndMenu_C|SetPlayer%20Display%20Name _endmenu "White"))))

(event EventOnStartWhiteTurn
  (Default|MovetoWhite (Variables|Default|GetBP_CameraTransition))
  (Default|SwitchSide (Variables|Default|GetWB_Countdown)))

(event EventOnStartBlackTurn
  (Default|MovetoBlack (Variables|Default|GetBP_CameraTransition))
  (Default|SwitchSide (Variables|Default|GetWB_Countdown)))

(event EventOnBlackWin
  (bind _endmenu (Utilities|CreateEndMenu)
    (:executeOut
      (Variables|/Game/HUD/EndMenu.EndMenu_C|SetPlayer%20Display%20Name _endmenu "Black"))))

(fn ConstructionScript)