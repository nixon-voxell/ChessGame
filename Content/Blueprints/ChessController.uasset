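; Chess player controller that shows the mouse cursor and copies the initial board state into its working state on BeginPlay.
; Every Tick, it traces under the cursor on the Visibility channel and prints the hit actor's name.
; SpawnChessTile creates a tile with a given material and board index, though nothing here calls it.
; SpawnChessPiece is an empty stub, with similar spawn logic left disconnected.
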(event EventBeginPlay
  (Variables|Default|SetbShowMouseCursor true)
  (Variables|Default|SetBoardState (Variables|Default|GetInitialBoardState)))

(event EventTick
  (params (DeltaSeconds :type Float%20%28single-precision%29))
  (Development|PrintString (Utilities|GetDisplayName (.HitActor (Collision|BreakHitResult (.HitResult (Game|Player|GetHitResultUnderCursorbyChannel "TraceTypeQuery1" true)))))))

(event Input|MouseEvents|LeftMouseButton
  (params (Key :type Key%20Structure :default "None")))

(fn ConstructionScript)

(fn SpawnChessTile
  (params (Position :type Vector) (Material :type Material%20Object%20Reference) (BoardIndex :type Integer))
  (bind _returnvalue (Game|SpawnActorfromClass "/Game/Blueprints/ChessTile.ChessTile_C" (Math|Conversions|ToTransform(Vector) Position) "Undefined" "MultiplyWithRoot" 0 0))
  (Rendering|Material|SetMaterial (Variables|/Game/Blueprints/ChessTile.ChessTile_C|GetCube _returnvalue) 0 Material)
  (Variables|/Game/Blueprints/ChessTile.ChessTile_C|SetBoardIndex _returnvalue BoardIndex))

(fn SpawnChessPiece
  (params (ChessPieceType :type Chess%20Piece%20Class%20Reference) (Position :type Vector) (Material :type Material%20Object%20Reference) (BoardIndex :type Integer)))