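; Pause Blueprint that toggles the game's paused state and pause menu.
; BeginPlay and the Pause input press share one toggle chain, so it also runs when play begins.
; The chain lazily creates and caches the PauseMenu widget, then branches on IsGamePaused to add or remove it from the viewport.
; Each branch sets global time dilation alongside the paused flag, zeroing it on pause and restoring it on resume.
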(event EventBeginPlay
  (Utilities|IsValid (Variables|Default|GetPauseMenuRef)
    (:Is%20Valid
      _)
    (:Is%20Not%20Valid
      (bind _returnvalue (UserInterface|CreateWidget "/Game/HUD/PauseMenu.PauseMenu_C"))
      (Variables|Default|SetPauseMenuRef _returnvalue)))
  (if (Game|IsGamePaused)
    (Utilities|Time|SetGlobalTimeDilation 1.0)
    (Widget|RemovefromParent (Variables|Default|GetPauseMenuRef))
    (Game|SetGamePaused false)
    (else
      (Utilities|Time|SetGlobalTimeDilation 0.0)
      (UserInterface|Viewport|AddtoViewport (Variables|Default|GetPauseMenuRef) 0)
      (Game|SetGamePaused true))))

(event Input|ActionEvents|InputActionPause
  (params (Key :type Key%20Structure :default "None"))
  (:Pressed
    (Utilities|IsValid (Variables|Default|GetPauseMenuRef)
      (:Is%20Valid
        _)
      (:Is%20Not%20Valid
        (bind _returnvalue (UserInterface|CreateWidget "/Game/HUD/PauseMenu.PauseMenu_C"))
        (Variables|Default|SetPauseMenuRef _returnvalue)))
    (if (Game|IsGamePaused)
      (Utilities|Time|SetGlobalTimeDilation 1.0)
      (Widget|RemovefromParent (Variables|Default|GetPauseMenuRef))
      (Game|SetGamePaused false)
      (else
        (Utilities|Time|SetGlobalTimeDilation 0.0)
        (UserInterface|Viewport|AddtoViewport (Variables|Default|GetPauseMenuRef) 0)
        (Game|SetGamePaused true)))))

(fn ConstructionScript)