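; ChessPiece is the Blueprint for a chess piece, pairing a static mesh with a box collision component.
; Its construction script sizes the box to half the mesh's scaled local bounds, so collision follows whichever mesh and scale are set.
; It then lifts the box by half the scaled height, which fits meshes with a base pivot.
; The event graph holds only disabled placeholder events, so no gameplay logic runs here.
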(event EventBeginPlay)

(event Collision|EventActorBeginOverlap
  (params (OtherActor :type Actor%20Object%20Reference)))

(event EventTick
  (params (DeltaSeconds :type Float%20%28single-precision%29)))

(fn ConstructionScript
  (bind _staticmesh (Variables|Default|GetStaticMesh))
  (bind _boxcollision (Variables|Default|GetBoxCollision))
  (bind (_min _max) (Components|StaticMesh|GetLocalBounds _staticmesh))
  (bind _relativescale3d (Variables|/Script/Engine.SceneComponent|GetRelativeScale3D _staticmesh))
  (bind _returnvalue (- _max _min))
  (bind _returnvalue_2 (* _relativescale3d _returnvalue))
  (Components|Box|SetBoxExtent _boxcollision (* _returnvalue_2 (Math|Conversions|ToVector(Float) 0.5)) true)
  (Transformation|AddLocalOffset _boxcollision (Math|Vector|MakeVector 0.0 0.0 (* (.Z (Math|Vector|BreakVector _returnvalue_2)) 0.5)) false true))