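; BP_PawnMovement is an unfinished Blueprint for chess pawn movement.
; On BeginPlay it confirms SelectedChessPiece is a PawnPiece through a cast, then line-traces from 400 units along +Y of the piece.
; A hit moves this actor, rather than the selected piece, to that offset; the trace has no end point set.
; A similar diagonal +X/+Y move exists but is disconnected and never runs.
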(event EventBeginPlay
  (bind _selectedchesspiece (Variables|Default|GetSelectedChessPiece))
  (bind _returnvalue (Transformation|GetActorLocation _selectedchesspiece))
  (bind (_x _y _z) (Class|KismetMathLibrary|BreakVector3f _returnvalue))
  (bind _returnvalue_2 (+ _y 4e+02))
  (bind _returnvalue_3 (Math|Vector|MakeVector _x _returnvalue_2 _z))
  ;[1 1 1] Incomplete
  (bind _ispawn (CallFunction|IsPawn _selectedchesspiece))
  (if _ispawn
    (bind _returnvalue_4 (Collision|LineTraceByChannel _returnvalue_3 "0, 0, 0" "TraceTypeQuery1" false 0 "None"))
    (if _returnvalue_4
      (Transformation|SetActorLocation _returnvalue_3 false false))))

(fn ConstructionScript)

(fn IsPawn
  (params (PawnToCheck :type Actor%20Object%20Reference))
  (Utilities|Casting|CastToPawnPiece PawnToCheck)
  (return true))