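; Chess board actor that spawns an 8x8 grid of alternating reflective tiles and the starting pieces on BeginPlay.
; The initial BoardState comes from the BoardStates DataTable as signed integers: magnitude selects a class from ChessPieceArrays, sign sets material and facing.
; Tiles and pieces spawn relative to the actor at Size spacing, each tagged with its BoardIndex.
; GetPieceIndexAtBoardIndex reads BoardState, while PositionToIndex holds only unconnected math.
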(event EventBeginPlay
  (CallFunction|InitializeChessTiles)
  (CallFunction|InitializeChessPieces))

(event EventTick
  (params (DeltaSeconds :type Float%20%28single-precision%29)))

(fn ConstructionScript
  (Variables|Default|SetHalfSize (* (Variables|Default|GetSize) 0.5)))

(fn SpawnChessTile
  (params (Position :type Vector) (Material :type Material%20Object%20Reference) (BoardIndex :type Integer))
  (bind _returnvalue (Game|SpawnActorfromClass "/Game/Blueprints/ChessTile.ChessTile_C" (Math|Transform|MakeRelativeTransform (Math|Conversions|ToTransform(Vector) Position) (Transformation|GetActorTransform)) "Undefined" "MultiplyWithRoot" 0 0))
  (Rendering|Material|SetMaterial (Variables|/Game/Blueprints/ChessTile.ChessTile_C|GetCube _returnvalue) 0 Material)
  (Variables|/Game/Blueprints/ChessTile.ChessTile_C|SetBoardIndex _returnvalue BoardIndex)
  (return _returnvalue))

(fn SpawnChessPiece
  (params (ChessPiece :type Chess%20Piece%20Class%20Reference) (Position :type Vector) (Rotation :type Rotator) (Material :type Material%20Object%20Reference) (BoardIndex :type Integer))
  (bind _returnvalue (Game|SpawnActorfromClass ChessPiece (Math|Transform|MakeRelativeTransform (Math|Transform|MakeTransform Position Rotation) (Transformation|GetActorTransform)) "Undefined" "MultiplyWithRoot" 0 0))
  (Rendering|Material|SetMaterial (Variables|/Game/Blueprints/ChessPiece.ChessPiece_C|GetStaticMesh _returnvalue) 0 Material)
  (Variables|/Game/Blueprints/ChessPiece.ChessPiece_C|SetBoardIndex _returnvalue BoardIndex)
  (return _returnvalue))

(fn InitializeChessTiles
  (for _index (range 0 7)
    (for _index_2 (range 0 7)
      (CallFunction|SpawnChessTile (* (Variables|Default|GetSize) (Math|Vector|MakeVector (Math|Conversions|ToFloat(Integer) _index_2) (Math|Conversions|ToFloat(Integer) _index) 0.0)) (select (Math|Conversions|ToBoolean(Integer) (Math|Integer|%(Integer) (+ _index _index_2) 2)) "/Game/Materials/BlackReflective.BlackReflective" "/Game/Materials/WhiteReflective.WhiteReflective") (+ (* _index 8) _index_2)))))

(fn InitializeChessPieces
  (bind _returnvalue (Utilities|GetDataTableRow "/Game/DataTables/BoardStates.BoardStates" "InitialState")
    (:then
      (Variables|Default|SetBoardState (Utilities|Struct|BreakBoardState _returnvalue))
      (for _index (range 0 7)
        (for _index_2 (range 0 7)
          (bind _returnvalue_2 (Utilities|GetDataTableRow "/Game/DataTables/ChessPieceArrays.ChessPieceArrays" "ChessPieceDefaultArray")
            (:then
              (if (Utilities|IsValidClass (Utilities|Array|Get(acopy) (Utilities|Struct|BreakChessPieceArray _returnvalue_2) (Math|Integer|Absolute(Integer) (Utilities|Array|Get(acopy) (Variables|Default|GetBoardState) (+ (* _index 8) _index_2)))))
                (CallFunction|SpawnChessPiece (Utilities|Array|Get(acopy) (Utilities|Struct|BreakChessPieceArray _returnvalue_2) (Math|Integer|Absolute(Integer) (Utilities|Array|Get(acopy) (Variables|Default|GetBoardState) (+ (* _index 8) _index_2)))) (+ (* (Variables|Default|GetSize) (Math|Vector|MakeVector (Math|Conversions|ToFloat(Integer) _index_2) (Math|Conversions|ToFloat(Integer) _index) 0.0)) "0.000000,0.000000,40.000000") (Math|Rotator|SelectRotator "0.000000,-90.000000,0.000000" "0.000000,90.000000,0.000000" (< (Class|KismetMathLibrary|SignOfInteger (Utilities|Array|Get(acopy) (Variables|Default|GetBoardState) (+ (* _index 8) _index_2))) 0)) (select (< (Class|KismetMathLibrary|SignOfInteger (Utilities|Array|Get(acopy) (Variables|Default|GetBoardState) (+ (* _index 8) _index_2))) 0) "/Game/Materials/Black.Black" "/Game/Materials/White.White") (+ (* _index 8) _index_2))))))))))

(fn GetPieceIndexatBoardIndex
  (params (BoardIndex :type Integer))
  (return (Utilities|Array|Get(acopy) (Variables|Default|GetBoardState) BoardIndex)))