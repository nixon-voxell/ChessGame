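; Chess board actor that procedurally builds the board and its starting pieces in the Construction Script, with no runtime logic.
; A 64-step loop lays out an 8x8 grid of tile meshes, choosing black or white by XOR of row and column parity.
; The StartFigures array selects one of six piece meshes per square, centered and colored by index.
; Pieces are scaled up, except types 3 and 4, whose scale nodes are disconnected.
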(event EventBeginPlay)

(event Collision|EventActorBeginOverlap
  (params (OtherActor :type Actor%20Object%20Reference)))

(event EventTick
  (params (DeltaSeconds :type Float%20%28single-precision%29)))

(fn ConstructionScript
  ;[1 1 1] Chess Board
  (for _index (range 0 63)
    (Utilities|FlowControl|Sequence
      (:then_0
        (bind _returnvalue (AddComponent|AddStaticMeshComponent false (Math|Conversions|ToTransform(Vector) (Math|Vector|MakeVector (Math|Conversions|ToFloat(Integer) (* (/ _index 8) 400)) (Math|Conversions|ToFloat(Integer) (* (Math|Integer|%(Integer) _index 8) 400)) 0.0))))
        (Rendering|Material|SetMaterial _returnvalue 0 (select (Math|Conversions|ToBoolean(Integer) (Class|KismetMathLibrary|XorIntInt (Math|Integer|%(Integer) _index 2) (Math|Integer|%(Integer) (/ _index 8) 2))) "/Game/Material/Black.Black" "/Game/Material/White.White")))
      (:then_1
        ;[1 1 1] Chess Pieces
        (switch int (Utilities|Array|Get(acopy) (Variables|Default|Getstart_figures) _index)
          (:1
            (bind _returnvalue_2 (AddComponent|AddStaticMeshComponent false (Math|Conversions|ToTransform(Vector) (+ (Math|Vector|MakeVector (Math|Conversions|ToFloat(Integer) (* (/ _index 8) 400)) (Math|Conversions|ToFloat(Integer) (* (Math|Integer|%(Integer) _index 8) 400)) 0.0) "200.000000,200.000000,0.000000"))))
            (Rendering|Material|SetMaterial _returnvalue_2 0 (select (> _index 30) "/Game/Material/Black.Black" "/Game/Material/White.White"))
            (Transformation|SetWorldScale3D _returnvalue_2 "50.000000,50.000000,50.000000"))
          (:2
            (bind _returnvalue_3 (AddComponent|AddStaticMeshComponent false (Math|Conversions|ToTransform(Vector) (+ (Math|Vector|MakeVector (Math|Conversions|ToFloat(Integer) (* (/ _index 8) 400)) (Math|Conversions|ToFloat(Integer) (* (Math|Integer|%(Integer) _index 8) 400)) 0.0) "200.000000,200.000000,0.000000"))))
            (Rendering|Material|SetMaterial _returnvalue_3 0 (select (> _index 30) "/Game/Material/Black.Black" "/Game/Material/White.White"))
            (Transformation|SetWorldScale3D _returnvalue_3 "50.000000,50.000000,50.000000"))
          (:3
            (bind _returnvalue_4 (AddComponent|AddStaticMeshComponent false (Math|Conversions|ToTransform(Vector) (+ (Math|Vector|MakeVector (Math|Conversions|ToFloat(Integer) (* (/ _index 8) 400)) (Math|Conversions|ToFloat(Integer) (* (Math|Integer|%(Integer) _index 8) 400)) 0.0) "200.000000,200.000000,0.000000"))))
            (Rendering|Material|SetMaterial _returnvalue_4 0 (select (> _index 30) "/Game/Material/Black.Black" "/Game/Material/White.White")))
          (:4
            (bind _returnvalue_5 (AddComponent|AddStaticMeshComponent false (Math|Conversions|ToTransform(Vector) (+ (Math|Vector|MakeVector (Math|Conversions|ToFloat(Integer) (* (/ _index 8) 400)) (Math|Conversions|ToFloat(Integer) (* (Math|Integer|%(Integer) _index 8) 400)) 0.0) "200.000000,200.000000,0.000000"))))
            (Rendering|Material|SetMaterial _returnvalue_5 0 (select (> _index 30) "/Game/Material/Black.Black" "/Game/Material/White.White")))
          (:5
            (bind _returnvalue_6 (AddComponent|AddStaticMeshComponent false (Math|Conversions|ToTransform(Vector) (+ (Math|Vector|MakeVector (Math|Conversions|ToFloat(Integer) (* (/ _index 8) 400)) (Math|Conversions|ToFloat(Integer) (* (Math|Integer|%(Integer) _index 8) 400)) 0.0) "200.000000,200.000000,0.000000"))))
            (Rendering|Material|SetMaterial _returnvalue_6 0 (select (> _index 30) "/Game/Material/Black.Black" "/Game/Material/White.White"))
            (Transformation|SetWorldScale3D _returnvalue_6 "50.000000,50.000000,50.000000"))
          (:6
            (bind _returnvalue_7 (AddComponent|AddStaticMeshComponent false (Math|Conversions|ToTransform(Vector) (+ (Math|Vector|MakeVector (Math|Conversions|ToFloat(Integer) (* (/ _index 8) 400)) (Math|Conversions|ToFloat(Integer) (* (Math|Integer|%(Integer) _index 8) 400)) 0.0) "200.000000,200.000000,0.000000"))))
            (Rendering|Material|SetMaterial _returnvalue_7 0 (select (> _index 30) "/Game/Material/Black.Black" "/Game/Material/White.White"))
            (Transformation|SetWorldScale3D _returnvalue_7 "50.000000,50.000000,50.000000")))))))