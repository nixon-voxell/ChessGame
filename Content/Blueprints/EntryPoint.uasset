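; EntryPoint is an actor Blueprint that runs the main menu's opening sequence on BeginPlay.
; It applies the resolution from a custom C++ GameUserSettings class and prints the resulting screen resolution as a check.
; It fades in by playing the Fade_Out widget's animation in reverse, switches the view to a camera and plays the CameraSlides_MainMenu sequence.
; After a short delay, it adds the Menu widget to the viewport.
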(event EventBeginPlay
  ;[1 1 1] Resolution Setting
  ;;[1 1 1] C++ Resolution Setting Custom
  (bind _returnvalue (Class|FixResolution|GetGameUserSettingsCustom))
  (Class|GameUserSettings|SetScreenResolution _returnvalue (Class|FixResolution|GetResolutionCustom _returnvalue))
  (Class|GameUserSettings|ApplyResolutionSettings _returnvalue false)
  (Class|GameUserSettings|ApplySettings _returnvalue true)
  ;[1 1 1] Resolution Testing & Check (Ignore)
  (bind _returnvalue_2 (Settings|GetGameUserSettings))
  (Development|PrintString (Utilities|String|ToString(Integer) (Class|GameUserSettings|GetScreenResolution _returnvalue_2)))
  ;[1 1 1] Fade In Effect
  (bind _returnvalue_3 (UserInterface|CreateWidget "/Game/HUD/Fade_Out.Fade_Out_C"))
  (UserInterface|Viewport|AddtoViewport _returnvalue_3 0)
  (UserInterface|Animation|PlayAnimation _returnvalue_3 (Variables|/Game/HUD/Fade_Out.Fade_Out_C|GetFadeIn _returnvalue_3) 0.0 1 "Reverse" 0.25 false)
  ;[1 1 1] Cinematic Camera Animation
  (Game|Player|SetViewTargetwithBlend (Game|GetPlayerController 0) (Variables|Default|GetCamera) 0.0 "VTBlend_Linear" 0.0 false)
  (bind _returnvalue_4 (Sequencer|Player|CreateLevelSequencePlayer "/Game/CameraSlides_MainMenu.CameraSlides_MainMenu"))
  (Sequencer|Player|Play _returnvalue_4 :!class /Script/MovieScene.MovieSceneSequencePlayer)
  (Utilities|FlowControl|Delay 2.5)
  ;[1 1 1] Show Menu UI
  (bind _returnvalue_5 (UserInterface|CreateWidget "/Game/HUD/Menu.Menu_C"))
  (UserInterface|Viewport|AddtoViewport _returnvalue_5 0))

(fn ConstructionScript)